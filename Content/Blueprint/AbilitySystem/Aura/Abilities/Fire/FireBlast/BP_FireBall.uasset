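; BP_FireBall is the Fire Blast ability's projectile, which flies outward, returns to a target actor and explodes near it.
; On the authority, an outgoing timeline lerps it to an apex along its forward vector, then a returning timeline homes on the target's current location.
; Within explode distance it calls OnHit, prepares radial damage, pitched knockback and death-impulse parameters for nearby live players except its owner, then destroys itself.
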(event EventStartOutgoingTimelines
  (bind _returnvalue (Components|GetOwner))
  (bind _array (Utilities|Array|MakeArray _returnvalue))
  (Networking|SwitchHasAuthority
    (:Authority
      (Variables|Default|SetInitialLocation (Transformation|GetActorLocation))
      (Variables|Default|SetApexLocation (+ (Variables|Default|GetInitialLocation) (* (Transformation|GetActorForwardVector) (Variables|Default|GetTravelDistance))))
      (bind _outgoingtrack (Timeline|Outgoing%20Timeline Play)
        (:Update
          (Transformation|SetActorLocation (Math|Vector|Lerp(Vector) (Variables|Default|GetInitialLocation) (Variables|Default|GetApexLocation) _outgoingtrack) false false))
        (:Finished
          (bind _returning_track (Timeline|Returning%20Timeline Play)
            (:Update
              (Transformation|SetActorLocation (Math|Vector|Lerp(Vector) (Variables|Default|GetApexLocation) (Transformation|GetActorLocation (Variables|Default|GetReturnToActor)) _returning_track) false false)
              (if (CallFunction|IsWinthinExplodeDistance)
                (Class|AuraProjectile|OnHit)
                (Class|AuraAbilitySystemLibrary|SetIsRadialDamageEffectParam (Variables|Default|GetExplosionDamageParams) true (Variables|Default|GetRadialDamageInnerRadius) (Variables|Default|GetRadialDamageOuterRadius) (Transformation|GetActorLocation))
                (Utilities|Array|Add _array self)
                (bind _outoverlappingactors (Class|AuraAbilitySystemLibrary|GetLivePlayersWithinRadius self _array (Variables|Default|GetRadialDamageOuterRadius) (Transformation|GetActorLocation)))
                (for _array_element _outoverlappingactors
                  (Class|AuraAbilitySystemLibrary|SetTargetEffectParamsASC (Variables|Default|GetExplosionDamageParams) (Ability|GetAbilitySystemComponent _array_element))
                  (Variables|Default|SetDirection (- (Transformation|GetActorLocation _array_element) (Transformation|GetActorLocation)))
                  (Class|AuraAbilitySystemLibrary|SetKnockbackDirection (Variables|Default|GetExplosionDamageParams) (Math|Vector|GetForwardVector (Math|Rotator|MakeRotator (.roll (Math|Rotator|MakeRotfromX (Variables|Default|GetDirection))) 45.0 (.yaw (Math|Rotator|MakeRotfromX (Variables|Default|GetDirection))))) (Variables|Default|GetKnockbackMagnitude))
                  (Class|AuraAbilitySystemLibrary|SetDeathImpulseDirection (Variables|Default|GetExplosionDamageParams) (Variables|Default|GetDirection) (Variables|Default|GetDeathImpulseMagnitude)))
                (Actor|DestroyActor)))))))))

(fn ConstructionScript)

(fn IsWinthinExplodeDistance
  (return (<= (Math|Vector|VectorLength (- (Transformation|GetActorLocation) (Transformation|GetActorLocation (Variables|Default|GetReturnToActor)))) (Variables|Default|GetExplodeDistance))))